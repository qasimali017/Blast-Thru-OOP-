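; Breakable brick for a ball-and-brick game that loses one strength point each time a Ball_BP hits it.
; Strength sets the cube's material, both in the construction script and after each non-fatal hit.
; At zero it plays an explosion and sound, then destroys itself.
; When no bricks remain, it reads the level number from LevelTracker_BP to open the next level, or show the win widget after level three.
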(event EventBeginPlay)

(event Collision|EventActorBeginOverlap
  (params (OtherActor :type Actor%20Object%20Reference)))

(event EventTick
  (params (DeltaSeconds :type Float%20%28single-precision%29)))

(event Collision|EventHit
  (params (MyComp :type Primitive%20Component%20Object%20Reference) (Other :type Actor%20Object%20Reference) (OtherComp :type Primitive%20Component%20Object%20Reference) (bSelfMoved :type Boolean) (HitLocation :type Vector :default "0, 0, 0") (HitNormal :type Vector :default "0, 0, 0") (NormalImpulse :type Vector :default "0, 0, 0") (Hit :type Hit%20Result%20Structure%20%28by%20ref%29))
  (Utilities|Casting|CastToBall_BP Other)
  (bind _result (Math|Integer|DecrementInt (Variables|Default|GetBrickStrength))
    (:%20%20
      (if (== _result 0)
        (Effects|SpawnEmitteratLocation "/Game/StarterContent/Particles/P_Explosion.P_Explosion" (Transformation|GetActorLocation))
        (Audio|PlaySoundatLocation "/Game/Music/break.break" (Transformation|GetActorLocation) "0, 0, 0" 1.0 1.0 0.0 0 0 0 0)
        (Actor|DestroyActor)
        (bind _outactors (Actor|GetAllActorsOfClass "Brick_BP_C"))
        (if (== (Utilities|Array|Length _outactors) 0)
          (bind _returnvalue (Actor|GetActorOfClass "/Game/Blueprints/LevelTracker_BP.LevelTracker_BP_C"))
          (switch int (Variables|/Game/Blueprints/LevelTracker_BP.LevelTracker_BP_C|Getlevelno _returnvalue)
            (:1
              (Game|OpenLevel(byObjectReference) "/Game/Maps/Level_2.Level_2"))
            (:2
              (Game|OpenLevel(byObjectReference) "/Game/Maps/Level_3.Level_3"))
            (:3
              (bind _returnvalue_2 (UserInterface|CreateWidget "/Game/Blueprints/Win_WBP.Win_WBP_C"))
              (UserInterface|Viewport|AddtoViewport _returnvalue_2 0))))
        (else
          (CallFunction|UpdateBrickColour))))))

(fn ConstructionScript
  (CallFunction|UpdateBrickColour))

(fn UpdateBrickColour
  (bind _cube (Variables|Default|GetCube))
  (switch int (Variables|Default|GetBrickStrength)
    (:1
      (Rendering|Material|SetMaterial _cube 0 "/Game/Materials/Yellow_inst.Yellow_inst"))
    (:2
      (Rendering|Material|SetMaterial _cube 0 "/Game/Materials/Red_inst.Red_inst"))
    (:3
      (Rendering|Material|SetMaterial _cube 0 "/Game/Materials/Green_inst.Green_inst"))
    (:4
      (Rendering|Material|SetMaterial _cube 0 "/Game/Materials/Brown_Glow.Brown_Glow"))))